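; BP_EnemyManager is a timed enemy spawner that creates BP_Enemy actors at its own location.
; Tick accumulates elapsed time in CurrentTime and, once it exceeds CreateTime, spawns an enemy regardless of collision and resets the counter.
; A disconnected CanSpawn check is left in the graph and never runs, so spawning depends on the timer alone.
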(event EventBeginPlay)

(event Collision|EventActorBeginOverlap
  (params (OtherActor :type Actor%20Object%20Reference)))

(event EventTick
  (params (DeltaSeconds :type Float%20%28single-precision%29))
  ;[0.15 0.15 0.15 0.5] 시간이 흐른다.
  (bind _output_get (Variables|Default|SetCurrentTime (+ DeltaSeconds (Variables|Default|GetCurrentTime))))
  ;[0.15 0.15 0.15 0.5] 생성시간이 됐으니까
  (if (> _output_get (Variables|Default|GetCreateTime))
    ;[0.15 0.15 0.15 0.5] 적생성
    (Game|SpawnActorfromClass "/Game/Blueprints/BP_Enemy.BP_Enemy_C" (Math|Transform|MakeTransform (Transformation|GetActorLocation) "0, 0, 0" "1.000000,1.000000,1.000000") "AlwaysSpawn" "MultiplyWithRoot" 0 0)
    (Variables|Default|SetCurrentTime 0.0)))

(fn ConstructionScript)