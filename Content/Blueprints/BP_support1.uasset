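; BP_support1 is a shooter actor that stays hidden for 18 seconds after play begins, then appears and fires repeatedly.
; It has collision enabled while hidden and disabled once visible, when a looping one-second timer starts calling FireBoss.
; Each FireBoss spawns a BP_Bullet at the world origin, another at the actor's transform through Fire, and plays a blaster sound.
; TakeDamage compares CurrentHP with itself, so any call destroys the actor.
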(event Custom|FireBoss
  (Game|SpawnActorfromClass "/Game/Blueprints/BP_Bullet.BP_Bullet_C" (Math|Transform|MakeTransform "0, 0, 0") "Undefined" "MultiplyWithRoot" 0 1 0)
  (CallFunction|Fire)
  (Audio|PlaySound2D "/Game/star-wars-blaster.star-wars-blaster" 1.0 1.0 0.0 0 0))

(event Collision|EventActorBeginOverlap
  (params (OtherActor :type Actor%20Object%20Reference)))

(event EventTick
  (params (DeltaSeconds :type Float%20%28single-precision%29)))

(event EventBeginPlay
  (Variables|Default|SetCurrentHP (Variables|Default|GetMaxHP))
  (Rendering|SetActorHiddenInGame true)
  (Collision|SetActorEnableCollision true)
  (Utilities|FlowControl|Delay 18.0)
  (Rendering|SetActorHiddenInGame false)
  (Collision|SetActorEnableCollision false)
  (Utilities|Time|SetTimerbyEvent (delegate Custom|FireBoss) 1.0 true))

(fn ConstructionScript)

(fn TakeDamage
  (params (Damage :type Float%20%28double-precision%29))
  (bind _output_get (Variables|Default|SetCurrentHP (- Damage (Variables|Default|GetCurrentHP))))
  (if (<= _output_get (Variables|Default|GetCurrentHP))
    (Actor|DestroyActor)))

(fn Fire
  (Game|SpawnActorfromClass "/Game/Blueprints/BP_Bullet.BP_Bullet_C" (Transformation|GetActorTransform) "Undefined" "MultiplyWithRoot" 0 1 0))